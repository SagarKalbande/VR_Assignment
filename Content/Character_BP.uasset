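; Character Blueprint with a camera and two display meshes, a Plane and a Cylinder, that show either left or right eye materials.
; The ChangeEye input flips both meshes between Left_Mat and Right_Mat, while ShowInputBuffer makes the Plane or the Cylinder visible, never both.
; The construction script forces a square camera aspect ratio and sets the ortho near clip plane, which BeginPlay prints for debugging.
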(event Custom|ShowInputBuffer
  (params (Visibility :type Boolean))
  (Rendering|SetVisibility (Variables|Default|GetPlane) Visibility false)
  (Rendering|SetVisibility (Variables|Default|GetCylinder) (not Visibility) false))

(event EventBeginPlay
  (Development|PrintString (Utilities|String|Append "Aspect Ratio is " (Utilities|String|ToString(Float) (Variables|/Script/Engine.CameraComponent|GetAspectRatio (Variables|Default|GetCamera)))) true true "(R=0.000000,G=0.660000,B=1.000000,A=1.000000)" 1e+01)
  (Development|PrintString (Utilities|String|Append "Near Clipping Plane is " (Utilities|String|ToString(Float) (Variables|/Script/Engine.CameraComponent|GetOrthoNearClipPlane (Variables|Default|GetCamera)))) true true "(R=0.000000,G=0.660000,B=1.000000,A=1.000000)" 1e+01))

(event Input|ActionEvents|InputActionChangeEye
  (params (Key :type Key%20Structure))
  (:Pressed
    (if (Variables|Default|GetCheck)
      (Rendering|Material|SetMaterial (Variables|Default|GetCylinder) 0 "/Game/Eye/right_Mat.right_Mat")
      (Variables|Default|SetCheck false)
      (else
        (Rendering|Material|SetMaterial (Variables|Default|GetCylinder) 0 "/Game/Eye/left_Mat.left_Mat")
        (Variables|Default|SetCheck true)))))

(fn ConstructionScript
  (bind _camera (Variables|Default|GetCamera))
  (Class|CameraComponent|SetAspectRatio _camera 1.0)
  (Variables|/Script/Engine.CameraComponent|SetOrthoNearClipPlane _camera 0.1))